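; Fluid system Blueprint that seeds a particle set and draws it with an instanced static mesh.
; BeginPlay spawns up to 500 motionless particles at random points in a box around the actor via SpawnParticle.
; The UpdateRenderData event clears all instances and rebuilds one small world-space instance per ParticleDatas entry.
; Neither simulation logic nor a call to UpdateRenderData appears in these graphs.
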(event `self.UpdateRenderData`
  (`InstancedStaticMeshComponent.ClearInstances` (`self.InstancedStaticMesh`))
  (for _array_element (`self.ParticleDatas`)
    (`InstancedStaticMeshComponent.AddInstanceWorldSpace` (`self.InstancedStaticMesh`) (`KismetMathLibrary.MakeTransform` (`.Location` (break `ParticleData` _array_element)) (struct) (0.01 0.01 0.01)))))

(event `self.ReceiveBeginPlay`
  (while (< (`self.SpawnedCount`) 500)
    (`self.SpawnParticle` (`KismetMathLibrary.RandomPointInBoundingBox` (`self.K2_GetActorLocation`) (100.0 100.0 100.0)))
    (`/Engine/EditorBlueprintResources/StandardMacros.IncrementInt` (`self.SpawnedCount`))))

(fn `UserConstructionScript`)